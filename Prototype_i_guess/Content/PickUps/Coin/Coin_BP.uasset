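; Coin pickup Blueprint for the 2D side-scroller that the player character collects by touching it.
; On overlap with the side-scroller character, it increments that character's coin count and immediately calls its save function.
; Each coin also adds a fixed increase to the character's max walk speed, then plays a pickup sound at its location and destroys itself.
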(event `self.ReceiveActorBeginOverlap`
  (params (OtherActor :type "Actor Object Reference"))
  (bind _as2dside_scroller_character (cast `/Game/Character/2DSideScrollerCharacter` OtherActor))
  (set `/Game/Character/2DSideScrollerCharacter.Coins_Amount` (+ (`/Game/Character/2DSideScrollerCharacter.Coins_Amount` _as2dside_scroller_character) 1) _as2dside_scroller_character)
  (`/Game/Character/2DSideScrollerCharacter.SaveGame` _as2dside_scroller_character)
  (bind _charactermovement (`Character.CharacterMovement` _as2dside_scroller_character))
  (set `CharacterMovementComponent.MaxWalkSpeed` (+ (`CharacterMovementComponent.MaxWalkSpeed` _charactermovement) 20.0) _charactermovement)
  (`GameplayStatics.PlaySoundAtLocation` "/Game/PickUps/Coin/CoinSound/CoinPickup_Cue.CoinPickup_Cue" (`self.K2_GetActorLocation` self) (struct) 1.0 1.0 0.0 null null null)
  (`self.K2_DestroyActor`))

(fn `UserConstructionScript`)